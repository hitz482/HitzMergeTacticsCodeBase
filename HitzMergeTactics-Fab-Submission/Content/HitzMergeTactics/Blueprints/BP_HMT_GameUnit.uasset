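; BP_HMT_GameUnit is a merge-tactics unit actor whose visuals come from the Unit Definition held by its UnitInstanceComponent.
; When a definition is applied, it loops that definition's idle animation on the mesh.
; On star level change, it swaps in a per-star skeletal mesh and uniform scale, then plays the merge sound at a socket or root location.
; Mesh and sound soft references are loaded with blocking loads.
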(event EventBeginPlay)

(event Collision|EventActorBeginOverlap
  (params (OtherActor :type Actor%20Object%20Reference)))

(event EventTick
  (params (DeltaSeconds :type Float%20%28single-precision%29)))

(event EventOnStarLevelChanged
  (params (OldStarLevel :type Integer) (NewStarLevel :type Integer))
  (bind _self self)
  (bind _unitinstancecomponent (Variables|Default|GetUnitInstanceComponent))
  (bind _returnvalue (Class|HMTUnitInstanceComponent|GetUnitDefinition _unitinstancecomponent))
  (bind (_boutfound _returnvalue_2) (Class|HMTUnitDefinition|GetMeshOverrideforStar _returnvalue NewStarLevel))
  (bind (_boutfound_2 _returnvalue_3) (Class|HMTUnitDefinition|GetScaleforStar _returnvalue NewStarLevel))
  (bind _returnvalue_4 (Class|HMTUnitDefinition|GetMergeSFXAsset _returnvalue))
  (Utilities|FlowControl|Sequence
    (:then_0
      (if _boutfound
        (bind _returnvalue_5 (Utilities|LoadAssetBlocking _returnvalue_2))
        (bind _asskeletal_mesh (Utilities|Casting|CastToSkeletalMesh _returnvalue_5))
        (Components|SkeletalMesh|SetSkeletalMeshAsset (Variables|Default|GetMeshComponent) _asskeletal_mesh)))
    (:then_1
      (if _boutfound_2
        (Transformation|SetActorScale3D _self (Math|Vector|MakeVector _returnvalue_3 _returnvalue_3 _returnvalue_3))))
    (:then_2
      (if (Utilities|IsValidSoftObjectReference _returnvalue_4)
        (bind _returnvalue_6 (Utilities|LoadAssetBlocking _returnvalue_4))
        (bind _assound_base (Utilities|Casting|CastToSoundBase _returnvalue_6))
        (Audio|PlaySoundatLocation _assound_base (Class|HMTUnitActor|GetSocketorRootLocation _self (Class|HMTUnitDefinition|GetMergeFXSocketName _returnvalue)) "0, 0, 0" 1.0 1.0 0.0 0 0 0 0)))))

(event EventOnUnitDefinitionApplied
  (bind _unitinstancecomponent (Variables|Default|GetUnitInstanceComponent))
  (bind _returnvalue (Class|HMTUnitInstanceComponent|GetUnitDefinition _unitinstancecomponent))
  (bind _returnvalue_2 (Class|HMTUnitDefinition|GetIdleAnim _returnvalue))
  (Utilities|IsValid _returnvalue_2
    (:Is%20Valid
      (Components|Animation|PlayAnimation (Variables|Default|GetMeshComponent) _returnvalue_2 true))))

(fn ConstructionScript)